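; VR stash inventory actor that builds its inventory on BeginPlay and shows it in pages.
; BeginPlay also binds events to left and right buttons and writes the current/max page counter to a text render.
; Motion controller overlaps on two box triggers step the page back or forward within zero and MaxPage, then refresh the counter and call UpdatePage.
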(event `self.ReceiveBeginPlay`
  (`self.ConstructInven`)
  (add `self.LeftButton` (`|CreateDelegate` :!event `Shuffle`))
  (add `self.RightButton` (`|CreateDelegate` :!event `SortAll`))
  (`TextRenderComponent.K2_SetText` (`self.TextRender4`) (`KismetTextLibrary.Conv_StringToText` (`KismetStringLibrary.Concat_StrStr` (`KismetStringLibrary.Conv_IntToString` (`self.CurrentPage`)) " / " (`KismetStringLibrary.Conv_IntToString` (`self.MaxPage`))))))

(event `self.Box3.OnComponentBeginOverlap`
  (params (OverlappedComponent :type "PrimitiveComponent Object Reference") (OtherActor :type "Actor Object Reference") (OtherComp :type "PrimitiveComponent Object Reference") (OtherBodyIndex :type Integer) (bFromSweep :type Boolean) (SweepResult :type "HitResult Structure (by ref)"))
  (bind _returnvalue (- (`self.CurrentPage`) 1))
  ;[1 1 1] 페이지 이동
  (cast `/Game/VirtualRealityBP/Blueprints/BP_MotionController` OtherActor)
  (if (>= _returnvalue 0)
    (set `self.CurrentPage` _returnvalue)
    (`TextRenderComponent.K2_SetText` (`self.TextRender4`) (`KismetTextLibrary.Conv_StringToText` (`KismetStringLibrary.Concat_StrStr` (`KismetStringLibrary.Conv_IntToString` (`self.CurrentPage`)) " / " (`KismetStringLibrary.Conv_IntToString` (`self.MaxPage`)))) :!label _label)
    (`self.UpdatePage`)))

(event `self.Box2.OnComponentBeginOverlap`
  (params (OverlappedComponent :type "PrimitiveComponent Object Reference") (OtherActor :type "Actor Object Reference") (OtherComp :type "PrimitiveComponent Object Reference") (OtherBodyIndex :type Integer) (bFromSweep :type Boolean) (SweepResult :type "HitResult Structure (by ref)"))
  (bind _returnvalue (+ (`self.CurrentPage`) 1))
  ;[1 1 1] 페이지 이동
  (cast `/Game/VirtualRealityBP/Blueprints/BP_MotionController` OtherActor)
  (if (<= _returnvalue (`self.MaxPage`))
    (set `self.CurrentPage` _returnvalue)
    (goto _label)))

(fn `UserConstructionScript`
  (`parent.UserConstructionScript`))