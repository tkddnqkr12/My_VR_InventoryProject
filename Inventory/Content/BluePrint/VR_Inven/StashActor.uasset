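; VR inventory stash actor with a physics-hinged lid that reacts to the player's presence.
; A MotionControllerPawn entering PlayerCheckArea triggers an upward impulse at the lid's handle, and leaving triggers one along the actor's forward vector.
; Tick maps the constraint twist to OpenRate, which scales the child actor with the lid.
; IsOpen sets near full open but never clears, as the clamped rate cannot drop below zero.
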(event `self.ReceiveTick`
  (params (DeltaSeconds :type "Float (single-precision)"))
  (bind _output_get (set `self.OpenRate` (`KismetMathLibrary.MapRangeClamped` (`PhysicsConstraintComponent.GetCurrentTwist` (`self.PhysicsConstraint`)) -120.0 0.0 1.0 0.0)))
  (bind _returnvalue (* _output_get 0.02))
  (`SceneComponent.SetWorldScale3D` (`self.ChildActor`) (`KismetMathLibrary.MakeVector` _returnvalue _returnvalue _returnvalue))
  (if (> (`self.OpenRate`) 0.9)
    (set `self.IsOpen` true)
    (elif (< (`self.OpenRate`) 0.0)
      (set `self.IsOpen` false))))

(event `self.PlayerCheckArea.OnComponentBeginOverlap`
  (params (OverlappedComponent :type "PrimitiveComponent Object Reference") (OtherActor :type "Actor Object Reference") (OtherComp :type "PrimitiveComponent Object Reference") (OtherBodyIndex :type Integer) (bFromSweep :type Boolean) (SweepResult :type "HitResult Structure (by ref)"))
  (bind _asmotion_controller_pawn (cast `/Game/VirtualRealityBP/Blueprints/MotionControllerPawn` OtherActor))
  (`PrimitiveComponent.AddImpulseAtLocation` (`self.Upper`) (0.0 0.0 20000.0) (`SceneComponent.K2_GetComponentLocation` (`self.HandlePoint`)) "None"))

(event `self.PlayerCheckArea.OnComponentEndOverlap`
  (params (OverlappedComponent :type "PrimitiveComponent Object Reference") (OtherActor :type "Actor Object Reference") (OtherComp :type "PrimitiveComponent Object Reference") (OtherBodyIndex :type Integer))
  (cast `/Game/VirtualRealityBP/Blueprints/MotionControllerPawn` OtherActor)
  (`PrimitiveComponent.AddImpulseAtLocation` (`self.Upper`) (* (`self.GetActorForwardVector`) 20000.0) (`SceneComponent.K2_GetComponentLocation` (`self.HandlePoint`)) "None"))

(fn `ConsturctStash`)

(fn `UserConstructionScript`)