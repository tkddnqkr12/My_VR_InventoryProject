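; A grabbable VR actor that carries an inventory and an equipment inventory as child actors.
; Pickup turns off physics on its Box and attaches it to the given component, and Drop restores physics and detaches it, both keeping world transforms.
; The construction script caches typed references to both child actors and passes its ItemDBManager to the inventory.
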(event `/Game/VirtualRealityBP/Blueprints/PickupActorInterface.Pickup`
  (params (AttachTo :type "SceneComponent Object Reference"))
  (bind _box (`self.Box`))
  (`PrimitiveComponent.SetSimulatePhysics` _box false)
  (`SceneComponent.K2_AttachToComponent` _box AttachTo "None" "KeepWorld" "KeepWorld" "KeepWorld" true))

(event `/Game/VirtualRealityBP/Blueprints/PickupActorInterface.Drop`
  (bind _box (`self.Box`))
  (`PrimitiveComponent.SetSimulatePhysics` _box true)
  (`SceneComponent.K2_DetachFromComponent` _box "KeepWorld" "KeepWorld" "KeepWorld" true))

(fn `UserConstructionScript`
  (`|ExecutionSequence`
    (:`then_0`
      (bind _asvr_inventory (cast `/Game/BluePrint/VR_Inven/VR_Inventory` (`ChildActorComponent.ChildActor` (`self.Inventory`))))
      (bind _output_get (set `self.InvenRef` _asvr_inventory))
      (set `/Game/BluePrint/VR_Inven/VR_Inventory.ItemDBManager` (`self.ItemDBManager`) _output_get))
    (:`then_1`
      (bind _asvr_equipment_inven (cast `/Game/BluePrint/VR_Inven/VR_EquipmentInven` (`ChildActorComponent.ChildActor` (`self.EquipInven`))))
      (set `self.EquipInvenRef` _asvr_equipment_inven))))