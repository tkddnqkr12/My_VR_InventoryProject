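; VR equipment inventory with head, chest, arm, weapon, waist and leg slots that totals the stats of equipped items.
; The construction script binds each child-actor VR_EquipSlot to this inventory with a location and ID.
; Setting or emptying a slot rebuilds damage, element, defense and resistance totals from scratch, then prints them on a TextRender.
; AddRes reads running totals by array index, so it assumes matching key order in both resistance maps.
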(event `self.ReceiveBeginPlay`)

(event `self.SetItemBySlotID`
  (params (SlotID :type Integer) (Item :type "/Game/BluePrint/VR_Inven/Items/ItemBase Object Reference") (Amount :type Integer))
  (`parent.SetItemBySlotID` SlotID Item Amount)
  (`self.UpdateStat`))

(event `self.MakeSlotEmpty`
  (params (SlotID :type Integer))
  (`parent.MakeSlotEmpty` SlotID)
  (`self.UpdateStat`))

(fn `AddRes`
  (params (Add :type "Map of /Game/BluePrint/VR_Inven/Items/Equipment/ElementalType Enum to Integer"))
  (bind _totalres (`self.TotalRes`))
  (bind _keys (`BlueprintMapLibrary.Map_Keys` Add))
  (for (_array_element _array_index) _keys
    (bind _values (`BlueprintMapLibrary.Map_Values` _totalres))
    (`BlueprintMapLibrary.Map_Add` _totalres _array_element (+ (`KismetArrayLibrary.Array_Get` _values _array_index) (`BlueprintMapLibrary.Map_Find` Add _array_element)))))

(fn `ResetStat`
  (bind _totalres (`self.TotalRes`))
  (set `self.TotalDamage` 0)
  (set `self.ElementalType` "NewEnumerator4")
  (set `self.ElementalDamage` 0)
  (set `self.TotalDef` 0)
  (`|ExecutionSequence`
    (:`then_0`
      (`BlueprintMapLibrary.Map_Add` _totalres "NewEnumerator0"))
    (:`then_1`
      (`BlueprintMapLibrary.Map_Add` _totalres "NewEnumerator1"))
    (:`then_2`
      (`BlueprintMapLibrary.Map_Add` _totalres "NewEnumerator2"))
    (:`then_3`
      (`BlueprintMapLibrary.Map_Add` _totalres "NewEnumerator3"))))

(fn `TextUpdate`
  (locals (TotalText :type String))
  (bind _totalres (`self.TotalRes`))
  (set `local.TotalText` (`KismetStringLibrary.Concat_StrStr` "Damage : " (`KismetStringLibrary.Conv_IntToString` (`self.TotalDamage`)) " \nType : " (`|GetEnumeratorNameAsString` (`self.ElementalType`)) " \nE_Damage : " (`KismetStringLibrary.Conv_IntToString` (`self.ElementalDamage`)) " \nDef : " (`KismetStringLibrary.Conv_IntToString` (`self.TotalDef`)) " \n== Res == \n"))
  (bind _keys (`BlueprintMapLibrary.Map_Keys` _totalres))
  (for (_array_element _array_index) _keys
    (bind _values (`BlueprintMapLibrary.Map_Values` _totalres))
    (set `local.TotalText` (`KismetStringLibrary.Concat_StrStr` (`local.TotalText`) (`|GetEnumeratorNameAsString` _array_element) " : " (`KismetStringLibrary.Conv_IntToString` (`KismetArrayLibrary.Array_Get` _values _array_index)) " \n")))
  (`TextRenderComponent.K2_SetText` (`self.TextRender2`) (`KismetTextLibrary.Conv_StringToText` (`local.TotalText`))))

(fn `UpdateStat`
  (bind _chestslot (`self.ChestSlot`))
  (bind _armslot (`self.ArmSlot`))
  (bind _waistslot (`self.WaistSlot`))
  (bind _legslot (`self.LegSlot`))
  (bind _weaponslot (`self.WeaponSlot`))
  (bind _headslot (`self.HeadSlot`))
  (bind _slotinfo_item (break `/Game/BluePrint/VR_Inven/SlotInfo` (`/Game/BluePrint/VR_Inven/VR_InvenSlot.SlotInfo` _waistslot)))
  (bind _slotinfo_item_2 (break `/Game/BluePrint/VR_Inven/SlotInfo` (`/Game/BluePrint/VR_Inven/VR_InvenSlot.SlotInfo` _weaponslot)))
  (bind _slotinfo_item_3 (break `/Game/BluePrint/VR_Inven/SlotInfo` (`/Game/BluePrint/VR_Inven/VR_InvenSlot.SlotInfo` _legslot)))
  (bind _slotinfo_item_4 (break `/Game/BluePrint/VR_Inven/SlotInfo` (`/Game/BluePrint/VR_Inven/VR_InvenSlot.SlotInfo` _armslot)))
  (bind _slotinfo_item_5 (break `/Game/BluePrint/VR_Inven/SlotInfo` (`/Game/BluePrint/VR_Inven/VR_InvenSlot.SlotInfo` _headslot)))
  (bind _slotinfo_item_6 (break `/Game/BluePrint/VR_Inven/SlotInfo` (`/Game/BluePrint/VR_Inven/VR_InvenSlot.SlotInfo` _chestslot)))
  (`self.ResetStat`)
  (`|ExecutionSequence`
    (:`then_0`
      (if (not (`/Game/BluePrint/VR_Inven/VR_InvenSlot.IsEmpty` _headslot))
        (bind _asitem_equipment_armor (cast `/Game/BluePrint/VR_Inven/Items/Equipment/ItemEquipment_Armor` _slotinfo_item_5))
        (set `self.TotalDef` (+ (`/Game/BluePrint/VR_Inven/Items/Equipment/ItemEquipment_Armor.Def` _asitem_equipment_armor) (`self.TotalDef`)))
        (`self.AddRes` (`/Game/BluePrint/VR_Inven/Items/Equipment/ItemEquipment_Armor.ElementalRes` _asitem_equipment_armor))))
    (:`then_1`
      (if (not (`/Game/BluePrint/VR_Inven/VR_InvenSlot.IsEmpty` _chestslot))
        (bind _asitem_equipment_armor_2 (cast `/Game/BluePrint/VR_Inven/Items/Equipment/ItemEquipment_Armor` _slotinfo_item_6))
        (set `self.TotalDef` (+ (`/Game/BluePrint/VR_Inven/Items/Equipment/ItemEquipment_Armor.Def` _asitem_equipment_armor_2) (`self.TotalDef`)))
        (`self.AddRes` (`/Game/BluePrint/VR_Inven/Items/Equipment/ItemEquipment_Armor.ElementalRes` _asitem_equipment_armor_2))))
    (:`then_2`
      (if (not (`/Game/BluePrint/VR_Inven/VR_InvenSlot.IsEmpty` _armslot))
        (bind _asitem_equipment_armor_3 (cast `/Game/BluePrint/VR_Inven/Items/Equipment/ItemEquipment_Armor` _slotinfo_item_4))
        (set `self.TotalDef` (+ (`/Game/BluePrint/VR_Inven/Items/Equipment/ItemEquipment_Armor.Def` _asitem_equipment_armor_3) (`self.TotalDef`)))
        (`self.AddRes` (`/Game/BluePrint/VR_Inven/Items/Equipment/ItemEquipment_Armor.ElementalRes` _asitem_equipment_armor_3))))
    (:`then_3`
      (if (not (`/Game/BluePrint/VR_Inven/VR_InvenSlot.IsEmpty` _waistslot))
        (bind _asitem_equipment_armor_4 (cast `/Game/BluePrint/VR_Inven/Items/Equipment/ItemEquipment_Armor` _slotinfo_item))
        (set `self.TotalDef` (+ (`/Game/BluePrint/VR_Inven/Items/Equipment/ItemEquipment_Armor.Def` _asitem_equipment_armor_4) (`self.TotalDef`)))
        (`self.AddRes` (`/Game/BluePrint/VR_Inven/Items/Equipment/ItemEquipment_Armor.ElementalRes` _asitem_equipment_armor_4))))
    (:`then_4`
      (if (not (`/Game/BluePrint/VR_Inven/VR_InvenSlot.IsEmpty` _legslot))
        (bind _asitem_equipment_armor_5 (cast `/Game/BluePrint/VR_Inven/Items/Equipment/ItemEquipment_Armor` _slotinfo_item_3))
        (set `self.TotalDef` (+ (`/Game/BluePrint/VR_Inven/Items/Equipment/ItemEquipment_Armor.Def` _asitem_equipment_armor_5) (`self.TotalDef`)))
        (`self.AddRes` (`/Game/BluePrint/VR_Inven/Items/Equipment/ItemEquipment_Armor.ElementalRes` _asitem_equipment_armor_5))))
    (:`then_5`
      (if (not (`/Game/BluePrint/VR_Inven/VR_InvenSlot.IsEmpty` _weaponslot))
        (bind _asitem_equipment_weapon (cast `/Game/BluePrint/VR_Inven/Items/Equipment/ItemEquipment_Weapon` _slotinfo_item_2))
        (set `self.TotalDamage` (+ (`/Game/BluePrint/VR_Inven/Items/Equipment/ItemEquipment_Weapon.Damage` _asitem_equipment_weapon) (`self.TotalDamage`)))
        (set `self.ElementalType` (`/Game/BluePrint/VR_Inven/Items/Equipment/ItemEquipment_Weapon.ElementalType` _asitem_equipment_weapon))
        (set `self.ElementalDamage` (+ (`self.ElementalDamage`) (`/Game/BluePrint/VR_Inven/Items/Equipment/ItemEquipment_Weapon.ElementalDamage` _asitem_equipment_weapon)))))
    (:`then_6`
      (`self.TextUpdate`))))

(fn `UserConstructionScript`
  (bind _returnvalue (`KismetArrayLibrary.Array_Length` (`self.Slots`)))
  (`parent.UserConstructionScript`)
  (`|ExecutionSequence`
    (:`then_0`
      (bind _asvr_equip_slot (cast `/Game/BluePrint/VR_Inven/VR_EquipSlot` (`ChildActorComponent.ChildActor` (`self.Head`))))
      (bind _output_get (set `self.HeadSlot` _asvr_equip_slot))
      (set `/Game/BluePrint/VR_Inven/VR_InvenSlot.Inventory` self _output_get)
      (set `/Game/BluePrint/VR_Inven/VR_EquipSlot.EquipLoc` "NewEnumerator0" _output_get)
      (set `/Game/BluePrint/VR_Inven/VR_InvenSlot.SlotID` 0 _output_get)
      (`KismetArrayLibrary.Array_Add` (`self.Slots`) _output_get))
    (:`then_1`
      (bind _asvr_equip_slot_2 (cast `/Game/BluePrint/VR_Inven/VR_EquipSlot` (`ChildActorComponent.ChildActor` (`self.Chest`))))
      (bind _output_get_2 (set `self.ChestSlot` _asvr_equip_slot_2))
      (set `/Game/BluePrint/VR_Inven/VR_InvenSlot.Inventory` self _output_get_2)
      (set `/Game/BluePrint/VR_Inven/VR_EquipSlot.EquipLoc` "NewEnumerator2" _output_get_2)
      (set `/Game/BluePrint/VR_Inven/VR_InvenSlot.SlotID` 1 _output_get_2)
      (`KismetArrayLibrary.Array_Add` (`self.Slots`) _output_get_2))
    (:`then_2`
      (bind _asvr_equip_slot_3 (cast `/Game/BluePrint/VR_Inven/VR_EquipSlot` (`ChildActorComponent.ChildActor` (`self.Arm`))))
      (bind _output_get_3 (set `self.ArmSlot` _asvr_equip_slot_3))
      (set `/Game/BluePrint/VR_Inven/VR_InvenSlot.Inventory` self _output_get_3)
      (set `/Game/BluePrint/VR_Inven/VR_EquipSlot.EquipLoc` "NewEnumerator3" _output_get_3)
      (set `/Game/BluePrint/VR_Inven/VR_InvenSlot.SlotID` 2 _output_get_3)
      (`KismetArrayLibrary.Array_Add` (`self.Slots`) _output_get_3))
    (:`then_3`
      (bind _asvr_equip_slot_4 (cast `/Game/BluePrint/VR_Inven/VR_EquipSlot` (`ChildActorComponent.ChildActor` (`self.Weapon`))))
      (bind _output_get_4 (set `self.WeaponSlot` _asvr_equip_slot_4))
      (set `/Game/BluePrint/VR_Inven/VR_InvenSlot.Inventory` self _output_get_4)
      (set `/Game/BluePrint/VR_Inven/VR_EquipSlot.EquipLoc` "NewEnumerator6" _output_get_4)
      (set `/Game/BluePrint/VR_Inven/VR_InvenSlot.SlotID` 3 _output_get_4)
      (`KismetArrayLibrary.Array_Add` (`self.Slots`) _output_get_4))
    (:`then_4`
      (bind _asvr_equip_slot_5 (cast `/Game/BluePrint/VR_Inven/VR_EquipSlot` (`ChildActorComponent.ChildActor` (`self.Waist`))))
      (bind _output_get_5 (set `self.WaistSlot` _asvr_equip_slot_5))
      (set `/Game/BluePrint/VR_Inven/VR_InvenSlot.Inventory` self _output_get_5)
      (set `/Game/BluePrint/VR_Inven/VR_EquipSlot.EquipLoc` "NewEnumerator4" _output_get_5)
      (set `/Game/BluePrint/VR_Inven/VR_InvenSlot.SlotID` 4 _output_get_5)
      (`KismetArrayLibrary.Array_Add` (`self.Slots`) _output_get_5))
    (:`then_5`
      (bind _asvr_equip_slot_6 (cast `/Game/BluePrint/VR_Inven/VR_EquipSlot` (`ChildActorComponent.ChildActor` (`self.Leg`))))
      (bind _output_get_6 (set `self.LegSlot` _asvr_equip_slot_6))
      (set `/Game/BluePrint/VR_Inven/VR_InvenSlot.Inventory` self _output_get_6)
      (set `/Game/BluePrint/VR_Inven/VR_EquipSlot.EquipLoc` "NewEnumerator5" _output_get_6)
      (set `/Game/BluePrint/VR_Inven/VR_InvenSlot.SlotID` 5 _output_get_6)
      (`KismetArrayLibrary.Array_Add` (`self.Slots`) _output_get_6))
    (:`then_6`
      (set `self.SlotNumPerPage` _returnvalue)
      (`KismetArrayLibrary.Array_Resize` (`self.AllSlots`) _returnvalue)
      (`self.UpdateStat`))))