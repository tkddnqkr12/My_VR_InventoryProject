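; VR_Stash is a VR crafting stash that combines items placed in its nine child-actor VR_InvenSlot slots.
; When a component tagged UI_Checker overlaps its Box, it searches the CombinationList data table for the first recipe whose resources the slots satisfy.
; It then subtracts those resources from the slots and adds the result item, looked up through ItemDBManager, to the first VR_Inventory actor found.
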(event `self.ReceiveTick`
  (params (DeltaSeconds :type "Float (single-precision)")))

(event `self.Box.OnComponentBeginOverlap`
  (params (OverlappedComponent :type "PrimitiveComponent Object Reference") (OtherActor :type "Actor Object Reference") (OtherComp :type "PrimitiveComponent Object Reference") (OtherBodyIndex :type Integer) (bFromSweep :type Boolean) (SweepResult :type "HitResult Structure (by ref)"))
  (if (`ActorComponent.ComponentHasTag` OtherComp "UI_Checker")
    (`self.Combine`)))

(fn `CheckAllTrue`
  (params (CheckList :type "Array of Boolean"))
  (returns (Result :type Boolean))
  (locals (Check :type Boolean))
  (for _array_element CheckList
    (if (not _array_element)
      (return false)))
  (return true))

(fn `CheckContainResource`
  (params (Element :type "/Game/BluePrint/VR_Inven/Items/CombinationElement Structure"))
  (returns (Success :type Boolean))
  (bind (_itemid _amount) (break `/Game/BluePrint/VR_Inven/Items/CombinationElement` Element))
  (for _array_element (`self.Slots`)
    (if (not (`/Game/BluePrint/VR_Inven/VR_InvenSlot.IsEmpty` _array_element))
      (bind (_slotinfo_item _slotinfo_amount) (break `/Game/BluePrint/VR_Inven/SlotInfo` (`/Game/BluePrint/VR_Inven/VR_InvenSlot.SlotInfo` _array_element)))
      (bind (_basicinfo_type _basicinfo_id) (break `/Game/BluePrint/VR_Inven/Items/Item_BasicInfo` (`/Game/BluePrint/VR_Inven/Items/ItemBase.BasicInfo` _slotinfo_item)))
      (if (and (== _basicinfo_id _itemid) (>= _slotinfo_amount _amount))
        (return true))))
  (return false))

(fn `Combine`
  (bind (_success _combinationrecipe) (`self.FindProperCombination`))
  (if _success
    (`self.ConsumeResource` _combinationrecipe)
    (bind _outactors (`GameplayStatics.GetAllActorsOfClass` "/Game/BluePrint/VR_Inven/VR_Inventory.VR_Inventory_C"))
    (bind (_resources _resultitemid _resultamount) (break `/Game/BluePrint/VR_Inven/Items/CombinationRecipe` _combinationrecipe))
    (`/Game/BluePrint/VR_Inven/VR_Inventory.AddItem` (`KismetArrayLibrary.Array_Get` _outactors) (`.Item` (`/Game/BluePrint/VR_Inven/Items/ItemDBManager.GetItemByID` (`self.ItemDBManager`) _resultitemid)) _resultamount)))

(fn `ConsumeResource`
  (params (Combination :type "/Game/BluePrint/VR_Inven/Items/CombinationRecipe Structure"))
  (for _array_element (`self.Slots`)
    (if (not (`/Game/BluePrint/VR_Inven/VR_InvenSlot.IsEmpty` _array_element))
      (for _array_element_2 (`.Resources_4_29D360E74C9048CE3C0EF89A8B2151EA` (break `/Game/BluePrint/VR_Inven/Items/CombinationRecipe` Combination))
        (bind (_itemid _amount) (break `/Game/BluePrint/VR_Inven/Items/CombinationElement` _array_element_2))
        (bind _slotinfo_item (break `/Game/BluePrint/VR_Inven/SlotInfo` (`/Game/BluePrint/VR_Inven/VR_InvenSlot.SlotInfo` _array_element)))
        (bind (_basicinfo_type _basicinfo_id) (break `/Game/BluePrint/VR_Inven/Items/Item_BasicInfo` (`/Game/BluePrint/VR_Inven/Items/ItemBase.BasicInfo` _slotinfo_item)))
        (if (== _itemid _basicinfo_id)
          (`/Game/BluePrint/VR_Inven/VR_InvenSlot.SubtractAmount` _array_element _amount)
          (break))))))

(fn `FindProperCombination`
  (returns (Success :type Boolean) (CombinationRecipe :type "/Game/BluePrint/VR_Inven/Items/CombinationRecipe Structure"))
  (locals (TotalList :type "Array of Boolean") (FindCombination :type "/Game/BluePrint/VR_Inven/Items/CombinationRecipe Structure") (Find :type Boolean))
  (bind _totallist (`local.TotalList`))
  (bind _outrownames (`DataTableFunctionLibrary.GetDataTableRowNames` "/Game/BluePrint/VR_Inven/Items/CombinationList.CombinationList"))
  (for _array_element _outrownames
    (bind _returnvalue (`|GetDataTableRow` "/Game/BluePrint/VR_Inven/Items/CombinationList.CombinationList" _array_element)
      (:`then`
        (for _array_element_2 (`.Resources_4_29D360E74C9048CE3C0EF89A8B2151EA` (break `/Game/BluePrint/VR_Inven/Items/CombinationRecipe` _returnvalue))
          (bind _success (`self.CheckContainResource` _array_element_2))
          (`KismetArrayLibrary.Array_Add` (`local.TotalList`) _success))
        (if (`self.CheckAllTrue` (`local.TotalList`))
          (set `local.FindCombination` _returnvalue)
          (set `local.Find` true)
          (break)
          (else
            (`KismetArrayLibrary.Array_Clear` _totallist)
            (`KismetArrayLibrary.Array_Resize` _totallist))))))
  (return (`local.Find`) (`local.FindCombination`)))

(fn `UserConstructionScript`
  (`|ExecutionSequence`
    (:`then_0`
      (bind _asvr_inven_slot (cast `/Game/BluePrint/VR_Inven/VR_InvenSlot` (`ChildActorComponent.ChildActor` (`self.Slot_0`))))
      (`KismetArrayLibrary.Array_Add` (`self.Slots`) _asvr_inven_slot))
    (:`then_1`
      (bind _asvr_inven_slot_2 (cast `/Game/BluePrint/VR_Inven/VR_InvenSlot` (`ChildActorComponent.ChildActor` (`self.Slot_1`))))
      (`KismetArrayLibrary.Array_Add` (`self.Slots`) _asvr_inven_slot_2))
    (:`then_2`
      (bind _asvr_inven_slot_3 (cast `/Game/BluePrint/VR_Inven/VR_InvenSlot` (`ChildActorComponent.ChildActor` (`self.Slot_2`))))
      (`KismetArrayLibrary.Array_Add` (`self.Slots`) _asvr_inven_slot_3))
    (:`then_3`
      (bind _asvr_inven_slot_4 (cast `/Game/BluePrint/VR_Inven/VR_InvenSlot` (`ChildActorComponent.ChildActor` (`self.Slot_3`))))
      (`KismetArrayLibrary.Array_Add` (`self.Slots`) _asvr_inven_slot_4))
    (:`then_4`
      (bind _asvr_inven_slot_5 (cast `/Game/BluePrint/VR_Inven/VR_InvenSlot` (`ChildActorComponent.ChildActor` (`self.Slot_4`))))
      (`KismetArrayLibrary.Array_Add` (`self.Slots`) _asvr_inven_slot_5))
    (:`then_5`
      (bind _asvr_inven_slot_6 (cast `/Game/BluePrint/VR_Inven/VR_InvenSlot` (`ChildActorComponent.ChildActor` (`self.Slot_5`))))
      (`KismetArrayLibrary.Array_Add` (`self.Slots`) _asvr_inven_slot_6))
    (:`then_6`
      (bind _asvr_inven_slot_7 (cast `/Game/BluePrint/VR_Inven/VR_InvenSlot` (`ChildActorComponent.ChildActor` (`self.Slot_6`))))
      (`KismetArrayLibrary.Array_Add` (`self.Slots`) _asvr_inven_slot_7))
    (:`then_7`
      (bind _asvr_inven_slot_8 (cast `/Game/BluePrint/VR_Inven/VR_InvenSlot` (`ChildActorComponent.ChildActor` (`self.Slot_7`))))
      (`KismetArrayLibrary.Array_Add` (`self.Slots`) _asvr_inven_slot_8))
    (:`then_8`
      (bind _asvr_inven_slot_9 (cast `/Game/BluePrint/VR_Inven/VR_InvenSlot` (`ChildActorComponent.ChildActor` (`self.Slot_8`))))
      (`KismetArrayLibrary.Array_Add` (`self.Slots`) _asvr_inven_slot_9))))