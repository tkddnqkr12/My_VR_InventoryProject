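; VR inventory actor that shows a paged grid of spawned, attached VR_InvenSlot actors, positioned by a pivot setting.
; AllSlots holds every page's data, and UpdatePage copies the current page into the visible slots.
; Adding stacks items by ID, recursing on overflow; older single-page add, sort and shuffle variants act directly on slots.
; Motion controllers overlapping two boxes trigger shuffle or ID sort, and BeginPlay adds random test items.
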(event `self.ReceiveEndPlay`
  (params (EndPlayReason :type "EEndPlayReason Enum" :default "Destroyed"))
  (`self.DestroySlots`))

(event `self.ReceiveBeginPlay`
  (`self.ConstructInven`)
  (`self.TestFunction`))

(event `TestFunction`
  (bind _itemdbmanager (`self.ItemDBManager`))
  (bind _ids (`/Game/BluePrint/VR_Inven/Items/ItemDBManager.GetAllStackableIDs` _itemdbmanager))
  (`self.MultiPages_AddItem` (`.Item` (`/Game/BluePrint/VR_Inven/Items/ItemDBManager.GetItemByID` _itemdbmanager (`KismetArrayLibrary.Array_Get` _ids (`KismetMathLibrary.RandomIntegerInRange` 0 (- (`KismetArrayLibrary.Array_Length` _ids) 1))))) (`KismetMathLibrary.RandomIntegerInRange` 1 99) :!label _label)
  (set `self.TestInt` (+ (`self.TestInt`) 1))
  (`KismetSystemLibrary.Delay` 0.5)
  (if (< (`self.TestInt`) 10)
    (goto _label)))

(event `self.Box.OnComponentBeginOverlap`
  (params (OverlappedComponent :type "PrimitiveComponent Object Reference") (OtherActor :type "Actor Object Reference") (OtherComp :type "PrimitiveComponent Object Reference") (OtherBodyIndex :type Integer) (bFromSweep :type Boolean) (SweepResult :type "HitResult Structure (by ref)"))
  (cast `/Game/VirtualRealityBP/Blueprints/BP_MotionController` OtherActor)
  (`self.MultiPage_Shuffle`))

(event `self.Box1.OnComponentBeginOverlap`
  (params (OverlappedComponent :type "PrimitiveComponent Object Reference") (OtherActor :type "Actor Object Reference") (OtherComp :type "PrimitiveComponent Object Reference") (OtherBodyIndex :type Integer) (bFromSweep :type Boolean) (SweepResult :type "HitResult Structure (by ref)"))
  (cast `/Game/VirtualRealityBP/Blueprints/BP_MotionController` OtherActor)
  (`self.SortAll`))

(fn `AddItem`
  (params (NewItem :type "/Game/BluePrint/VR_Inven/Items/ItemBase Object Reference") (Amount :type Integer))
  (locals (BeforeAmount :type Integer))
  (bind (_type _id _name _description _category _rarity _maxcapacity) (break `/Game/BluePrint/VR_Inven/Items/Item_BasicInfo` (`/Game/BluePrint/VR_Inven/Items/ItemBase.BasicInfo` NewItem)))
  (if (> Amount 0)
    ;[1 1 1] 인벤토리에 아이템이 존재하는지 확인
    (bind (_exsist _slotid) (`self.CheckItemExsiting` NewItem))
    (if _exsist
      ;[1 1 1] 존재할 경우 해당 슬롯에 아이템 추가
      (`self.AddItemToSlot` (`.Slot` (`self.GetSlotByID` _slotid)) NewItem Amount)
      (else
        ;[1 1 1] 존재하지 않을 경우
        ;;[1 1 1] 빈슬롯 확인
        (bind (_success _slotid_2) (`self.GetEmptySlot`))
        (if _success
          ;;[1 1 1] 새로 추가될 아이템의 갯수가 최대갯수를 넘는지 확인
          (if (<= Amount _maxcapacity)
            (bind (_success_2 _slot) (`self.GetSlotByID` _slotid_2))
            ;;[0 0.7457 1] 안넘을 경우 그냥 추가
            (`/Game/BluePrint/VR_Inven/VR_InvenSlot.SetItemAndAmount` _slot NewItem Amount)
            (else
              ;;[1 0.06651 0] 넘을 경우 다른칸에 더불어 추가
              (`/Game/BluePrint/VR_Inven/VR_InvenSlot.SetItemAndAmount` _slot NewItem _maxcapacity)
              (`self.AddItem` NewItem (- Amount _maxcapacity))))
          (else
            ;;[1 1 1] 빈슬롯이 없을 경우
            (`KismetSystemLibrary.PrintString` "No Vacancy")))))))

(fn `AddItemToSlot`
  (params (SpecificSlot :type "/Game/BluePrint/VR_Inven/VR_InvenSlot Object Reference") (Item :type "/Game/BluePrint/VR_Inven/Items/ItemBase Object Reference") (Amount :type Integer))
  (locals (BeforeAmount :type Integer))
  (bind (_slotinfo_item _slotinfo_amount) (break `/Game/BluePrint/VR_Inven/SlotInfo` (`/Game/BluePrint/VR_Inven/VR_InvenSlot.SlotInfo` SpecificSlot)))
  (bind (_type _id _name _description _category _rarity _maxcapacity) (break `/Game/BluePrint/VR_Inven/Items/Item_BasicInfo` (`/Game/BluePrint/VR_Inven/Items/ItemBase.BasicInfo` Item)))
  (bind (_type_2 _id_2 _name_2 _description_2 _category_2 _rarity_2 _maxcapacity_2) (break `/Game/BluePrint/VR_Inven/Items/Item_BasicInfo` (`/Game/BluePrint/VR_Inven/Items/ItemBase.BasicInfo` _slotinfo_item)))
  ;[1 1 1] 해당 슬롯이 꽉찼는지 확인
  (if (`/Game/BluePrint/VR_Inven/VR_InvenSlot.IsFull` SpecificSlot)
    ;[1 0.466 0] 꽉 찼을 경우
    ;;[1 1 1] 동일 아이템 다른 슬롯을 찾음
    (bind (_success _id_3) (`self.GetNotFullSlot` Item))
    (if _success
      ;;[1 1 1] 찾았을 경우 그 슬롯에 더해줌
      (`self.AddItemToSlot` (`.Slot` (`self.GetSlotByID` _id_3)) Item Amount)
      (else
        ;;[1 1 1] 빈슬롯 찾음
        (bind (_success_2 _slotid) (`self.GetEmptySlot`))
        (if _success_2
          ;;[1 1 1] 빈슬롯에 더할 때 최대갯수를 넘는지 확인
          (if (> _maxcapacity Amount)
            (bind (_success_3 _slot) (`self.GetSlotByID` _slotid))
            ;;[1 1 1] 안넘을 경우 그대로 아이템 and 갯수 설정
            (`/Game/BluePrint/VR_Inven/VR_InvenSlot.SetItemAndAmount` _slot Item Amount)
            (else
              ;;[1 1 1] 넘을 경우 일단 빈슬롯에 최대갯수로 채우고 남은 갯수만큼 다시 더해줌
              (`/Game/BluePrint/VR_Inven/VR_InvenSlot.SetItemAndAmount` _slot Item _maxcapacity)
              (`self.AddItem` Item (- Amount _maxcapacity)))))))
    (else
      ;[1 0 0.4724] 꽉 차지 않았을 경우
      ;;[1 1 1] 더했을 때 최대갯수를 넘는지 안넘는지 확인
      (if (> (+ _slotinfo_amount Amount) _maxcapacity_2)
        ;;[1 1 1] 넘을 경우 해당슬롯을 최대갯수로 만들어주고 나머지 갯수만큼 다시 추가
        (bind _output_get (set `local.BeforeAmount` _slotinfo_amount))
        (`/Game/BluePrint/VR_Inven/VR_InvenSlot.SetAmount` SpecificSlot _maxcapacity_2)
        (`self.AddItem` Item (- (+ _output_get Amount) _maxcapacity_2))
        (else
          ;;[1 1 1] 안넘을 경우 갯수 추가
          (`/Game/BluePrint/VR_Inven/VR_InvenSlot.AddAmount` SpecificSlot Amount))))))

(fn `CalcSlotID`
  (params (Slot :type "/Game/BluePrint/VR_Inven/VR_InvenSlot Object Reference"))
  (returns (CalcID :type Integer))
  (return (+ (`/Game/BluePrint/VR_Inven/VR_InvenSlot.SlotID` Slot) (* (`self.SlotNumPerPage`) (`self.CurrentPage`)))))

(fn `CheckItemExsiting`
  (params (CheckItem :type "/Game/BluePrint/VR_Inven/Items/ItemBase Object Reference"))
  (returns (Exsist :type Boolean) (SlotID :type Integer))
  (for (_array_element _array_index) (`self.Slots`)
    (if (`/Game/BluePrint/VR_Inven/VR_InvenSlot.IsEmpty` _array_element)
      _
      (elif (== (`.ID_2_604D97914D5493F688E27BACE8A49872` (break `/Game/BluePrint/VR_Inven/Items/Item_BasicInfo` (`/Game/BluePrint/VR_Inven/Items/ItemBase.BasicInfo` (`.Item_3_7DCF77FE4EC0FE901CF57A9A3899E4A2` (break `/Game/BluePrint/VR_Inven/SlotInfo` (`/Game/BluePrint/VR_Inven/VR_InvenSlot.SlotInfo` _array_element)))))) (`.ID_2_604D97914D5493F688E27BACE8A49872` (break `/Game/BluePrint/VR_Inven/Items/Item_BasicInfo` (`/Game/BluePrint/VR_Inven/Items/ItemBase.BasicInfo` CheckItem))))
        (return true _array_index))))
  (return false -1))

(fn `ConstructInven`
  (locals (SlotRef :type "/Game/BluePrint/VR_Inven/VR_InvenSlot Object Reference"))
  (bind (_returnvalue_location _returnvalue_rotation _returnvalue_scale) (`KismetMathLibrary.BreakTransform` (`self.GetTransform`)))
  (bind _slotref (`local.SlotRef`))
  (`self.SetPivot` (`self.Pivot`))
  (for _index (range (`self.Row`))
    (for _index_2 (range (`self.Colum`))
      (bind _returnvalue (`|SpawnActorFromClass` "/Game/BluePrint/VR_Inven/VR_InvenSlot.VR_InvenSlot_C" (`KismetMathLibrary.MakeTransform` (0.0 0.0 0.0) (struct) _returnvalue_scale) "AlwaysSpawn" "OverrideRootScale" null self))
      (bind _output_get (set `local.SlotRef` _returnvalue))
      (`self.K2_AttachToActor` _output_get self "None" "KeepWorld" "KeepRelative" "KeepWorld" false)
      (`self.K2_SetActorRelativeLocation` _slotref (`KismetMathLibrary.MakeVector` 0.0 (+ (`self.Start_X`) (* (* _index_2 (`self.Padding_X`)) -1.0)) (+ (`self.Start_Y`) (* (* _index (`self.Padding_Y`)) -1.0))) false false)
      (set `/Game/BluePrint/VR_Inven/VR_InvenSlot.SlotID` (+ _index_2 (* _index (`self.Colum`))) _slotref)
      (`KismetArrayLibrary.Array_Add` (`self.Slots`) _slotref)))
  (bind _output_get_2 (set `self.SlotNumPerPage` (* (`self.Colum`) (`self.Row`))))
  (`KismetArrayLibrary.Array_Resize` (`self.AllSlots`) (* _output_get_2 (`self.MaxPage`))))

(fn `DestroySlots`
  (for _array_element (`self.Slots`)
    (`self.K2_DestroyActor` _array_element)))

(fn `GetEmptySlot`
  (returns (Success :type Boolean) (SlotID :type Integer))
  (for (_array_element _array_index) (`self.Slots`)
    (if (`/Game/BluePrint/VR_Inven/VR_InvenSlot.IsEmpty` _array_element)
      (return true _array_index)))
  (return false -1))

(fn `GetNotFullSlot`
  (params (Item :type "/Game/BluePrint/VR_Inven/Items/ItemBase Object Reference"))
  (returns (Success :type Boolean) (ID :type Integer))
  (locals (Find :type Boolean) (Result :type Integer :default 0))
  (for _array_element (`self.Slots`)
    (bind _slotinfo_item (break `/Game/BluePrint/VR_Inven/SlotInfo` (`/Game/BluePrint/VR_Inven/VR_InvenSlot.SlotInfo` _array_element)))
    (if (== _slotinfo_item Item)
      (if (not (`/Game/BluePrint/VR_Inven/VR_InvenSlot.IsFull` _array_element))
        (set `local.Find` true)
        (set `local.Result` (`/Game/BluePrint/VR_Inven/VR_InvenSlot.SlotID` _array_element)))))
  (return (`local.Find`) (`local.Result`)))

(fn `GetSlotByID`
  (params (ID :type Integer))
  (returns (Success :type Boolean) (Slot :type "/Game/BluePrint/VR_Inven/VR_InvenSlot Object Reference"))
  (locals (Find :type Boolean) (Result :type "/Game/BluePrint/VR_Inven/VR_InvenSlot Object Reference"))
  (for _array_element (`self.Slots`)
    (if (== (`/Game/BluePrint/VR_Inven/VR_InvenSlot.SlotID` _array_element) ID)
      (set `local.Find` true)
      (set `local.Result` _array_element)
      (break)))
  (return (`local.Find`) (`local.Result`)))

(fn `MakeSlotEmpty`
  (params (SlotID :type Integer))
  (`KismetArrayLibrary.Array_Set` (`self.AllSlots`) SlotID (make `/Game/BluePrint/VR_Inven/SlotInfo` null))
  (`self.UpdatePage`))

(fn `MultiPage_Shuffle`
  (locals (Infos :type "Array of /Game/BluePrint/VR_Inven/SlotInfo Structure"))
  (`KismetArrayLibrary.Array_Shuffle` (`self.AllSlots`))
  (`self.UpdatePage`))

(fn `MultiPages_AddItem`
  (params (NewItem :type "/Game/BluePrint/VR_Inven/Items/ItemBase Object Reference") (Amount :type Integer))
  (bind (_basicinfo_type _basicinfo_id _basicinfo_name _basicinfo_description _basicinfo_category _basicinfo_rarity _basicinfo_maxcapacity) (break `/Game/BluePrint/VR_Inven/Items/Item_BasicInfo` (`/Game/BluePrint/VR_Inven/Items/ItemBase.BasicInfo` NewItem)))
  (if (> Amount 0)
    (bind (_success _slotid) (`self.MultiPages_CheckItemExsiting` NewItem))
    (if _success
      (`self.MultiPages_AddItemToSlot` _slotid NewItem Amount)
      (else
        (bind (_success_2 _slotid_2) (`self.MultiPages_GetEmptySlot`))
        (if _success_2
          (if (<= Amount _basicinfo_maxcapacity)
            (`self.SetItemBySlotID` _slotid_2 NewItem Amount)
            (else
              (`self.SetItemBySlotID` _slotid_2 NewItem _basicinfo_maxcapacity)
              (`self.MultiPages_AddItem` NewItem (- Amount _basicinfo_maxcapacity))))
          (else
            (`KismetSystemLibrary.PrintString` "NoVacancy")))))))

(fn `MultiPages_AddItemToSlot`
  (params (SlotID :type Integer) (Item :type "/Game/BluePrint/VR_Inven/Items/ItemBase Object Reference") (Amount :type Integer))
  (locals (BeforeAmount :type Integer))
  (bind (_basicinfo_type _basicinfo_id _basicinfo_name _basicinfo_description _basicinfo_category _basicinfo_rarity _basicinfo_maxcapacity) (break `/Game/BluePrint/VR_Inven/Items/Item_BasicInfo` (`/Game/BluePrint/VR_Inven/Items/ItemBase.BasicInfo` Item)))
  (bind _item (`KismetArrayLibrary.Array_Get` (`self.AllSlots`) SlotID))
  (bind (_item_2 _amount) (break `/Game/BluePrint/VR_Inven/SlotInfo` _item))
  (bind _returnvalue (+ _amount Amount))
  (bind (_basicinfo_type_2 _basicinfo_id_2 _basicinfo_name_2 _basicinfo_description_2 _basicinfo_category_2 _basicinfo_rarity_2 _basicinfo_maxcapacity_2) (break `/Game/BluePrint/VR_Inven/Items/Item_BasicInfo` (`/Game/BluePrint/VR_Inven/Items/ItemBase.BasicInfo` _item_2)))
  (if (`/Game/BluePrint/VR_Inven/Items/CommonItemFunction.IsFull` _item)
    (bind (_success _slotid) (`self.MultiPages_GetNotFullSlot` Item))
    (if _success
      (`self.MultiPages_AddItemToSlot` _slotid Item Amount)
      (else
        (bind (_success_2 _slotid_2) (`self.MultiPages_GetEmptySlot`))
        (if _success_2
          (if (> _basicinfo_maxcapacity Amount)
            (`self.SetItemBySlotID` _slotid_2 Item Amount)
            (else
              (`self.SetItemBySlotID` _slotid_2 Item _basicinfo_maxcapacity)
              (`self.MultiPages_AddItem` Item (- Amount _basicinfo_maxcapacity)))))))
    (elif (> _returnvalue _basicinfo_maxcapacity_2)
      (set `local.BeforeAmount` _amount)
      (`self.SetItemBySlotID` SlotID Item _basicinfo_maxcapacity_2)
      (`self.MultiPages_AddItem` Item (- (+ (`local.BeforeAmount`) Amount) _basicinfo_maxcapacity_2))
      (else
        (`self.SetItemBySlotID` SlotID Item _returnvalue)))))

(fn `MultiPages_CheckItemExsiting`
  (params (FindItem :type "/Game/BluePrint/VR_Inven/Items/ItemBase Object Reference"))
  (returns (Success :type Boolean) (SlotID :type Integer))
  (for (_array_element _array_index) (`self.AllSlots`)
    (if (`/Game/BluePrint/VR_Inven/Items/CommonItemFunction.IsEmpty` _array_element)
      _
      (elif (== (`.ID_2_604D97914D5493F688E27BACE8A49872` (break `/Game/BluePrint/VR_Inven/Items/Item_BasicInfo` (`/Game/BluePrint/VR_Inven/Items/ItemBase.BasicInfo` (`.Item_3_7DCF77FE4EC0FE901CF57A9A3899E4A2` (break `/Game/BluePrint/VR_Inven/SlotInfo` _array_element))))) (`.ID_2_604D97914D5493F688E27BACE8A49872` (break `/Game/BluePrint/VR_Inven/Items/Item_BasicInfo` (`/Game/BluePrint/VR_Inven/Items/ItemBase.BasicInfo` FindItem))))
        (return true _array_index))))
  (return false -1))

(fn `MultiPages_GetEmptySlot`
  (returns (Success :type Boolean) (SlotID :type Integer))
  (for (_array_element _array_index) (`self.AllSlots`)
    (if (`/Game/BluePrint/VR_Inven/Items/CommonItemFunction.IsEmpty` _array_element)
      (return true _array_index)))
  (return false -1))

(fn `MultiPages_GetNotFullSlot`
  (params (CheckItem :type "/Game/BluePrint/VR_Inven/Items/ItemBase Object Reference"))
  (returns (Success :type Boolean) (SlotID :type Integer))
  (bind (_basicinfo_type _basicinfo_id) (break `/Game/BluePrint/VR_Inven/Items/Item_BasicInfo` (`/Game/BluePrint/VR_Inven/Items/ItemBase.BasicInfo` CheckItem)))
  (for (_array_element _array_index) (`self.AllSlots`)
    (if (not (`/Game/BluePrint/VR_Inven/Items/CommonItemFunction.IsEmpty` _array_element))
      (bind (_basicinfo_type_2 _basicinfo_id_2) (break `/Game/BluePrint/VR_Inven/Items/Item_BasicInfo` (`/Game/BluePrint/VR_Inven/Items/ItemBase.BasicInfo` (`.Item_3_7DCF77FE4EC0FE901CF57A9A3899E4A2` (break `/Game/BluePrint/VR_Inven/SlotInfo` _array_element)))))
      (if (== _basicinfo_id_2 _basicinfo_id)
        (if (not (`/Game/BluePrint/VR_Inven/Items/CommonItemFunction.IsFull` _array_element))
          (return true _array_index)))))
  (return false -1))

(fn `SetItemBySlotID`
  (params (SlotID :type Integer) (Item :type "/Game/BluePrint/VR_Inven/Items/ItemBase Object Reference") (Amount :type Integer))
  (locals (SlotInfo :type "/Game/BluePrint/VR_Inven/SlotInfo Structure"))
  (bind _structout (setmembers `/Game/BluePrint/VR_Inven/SlotInfo` :`StructRef` (`local.SlotInfo`) :`Item` Item :`Amount` Amount))
  (`KismetArrayLibrary.Array_Set` (`self.AllSlots`) SlotID _structout)
  (`self.UpdatePage`))

(fn `SetPivot`
  (params (Pivot :type "/Game/BluePrint/VR_Inven/InvenPivot Enum"))
  (bind _padding_x (`self.Padding_X`))
  (bind _padding_y (`self.Padding_Y`))
  (bind _returnvalue (* (`self.Colum`) _padding_x))
  (bind _returnvalue_2 (* (`self.Row`) _padding_y))
  (bind _output_get (set `self.Pivot` Pivot))
  (switch `/Game/BluePrint/VR_Inven/InvenPivot` _output_get
    (:`NewEnumerator0`
      (`|ExecutionSequence`
        (:`then_0`
          ;[1 1 1] Left
          (set `self.Start_X` 0.0 :!label _label))
        (:`then_1`
          ;[1 1 1] Top
          (set `self.Start_Y` 0.0 :!label _label_2))))
    (:`NewEnumerator1`
      (`|ExecutionSequence`
        (:`then_0`
          ;[1 1 1] Center
          (set `self.Start_X` (- (* _returnvalue 0.5) (* _padding_x 0.5)) :!label _label_3))
        (:`then_1`
          (goto _label_2))))
    (:`NewEnumerator2`
      (`|ExecutionSequence`
        (:`then_0`
          ;[1 1 1] Right
          (set `self.Start_X` (- _returnvalue _padding_x) :!label _label_4))
        (:`then_1`
          (goto _label_2))))
    (:`NewEnumerator3`
      (`|ExecutionSequence`
        (:`then_0`
          (goto _label))
        (:`then_1`
          ;[1 1 1] Middle
          (set `self.Start_Y` (- (* _returnvalue_2 0.5) (* _padding_y 0.5)) :!label _label_5))))
    (:`NewEnumerator4`
      (`|ExecutionSequence`
        (:`then_0`
          (goto _label_3))
        (:`then_1`
          (goto _label_5))))
    (:`NewEnumerator5`
      (`|ExecutionSequence`
        (:`then_0`
          (goto _label_4))
        (:`then_1`
          (goto _label_5))))
    (:`NewEnumerator6`
      (`|ExecutionSequence`
        (:`then_0`
          (goto _label))
        (:`then_1`
          ;[1 1 1] Bottom
          (set `self.Start_Y` (- _returnvalue_2 _padding_y) :!label _label_6))))
    (:`NewEnumerator7`
      (`|ExecutionSequence`
        (:`then_0`
          (goto _label_3))
        (:`then_1`
          (goto _label_6))))
    (:`NewEnumerator8`
      (`|ExecutionSequence`
        (:`then_0`
          (goto _label_4))
        (:`then_1`
          (goto _label_6))))))

(fn `Shuffle`
  (locals (Infos :type "Array of /Game/BluePrint/VR_Inven/SlotInfo Structure"))
  (bind _infos (`local.Infos`))
  (for _array_element (`self.Slots`)
    (`KismetArrayLibrary.Array_Add` (`local.Infos`) (`/Game/BluePrint/VR_Inven/VR_InvenSlot.SlotInfo` _array_element)))
  (for _array_element_2 (`self.Slots`)
    (`/Game/BluePrint/VR_Inven/VR_InvenSlot.MakeEmpty` _array_element_2))
  (`KismetArrayLibrary.Array_Shuffle` _infos)
  (for (_array_element_3 _array_index) _infos
    (bind (_item _amount) (break `/Game/BluePrint/VR_Inven/SlotInfo` _array_element_3))
    (`/Game/BluePrint/VR_Inven/VR_InvenSlot.SetItemAndAmount` (`KismetArrayLibrary.Array_Get` (`self.Slots`) _array_index) _item _amount)))

(fn `Sort`
  (locals (BeforeInfo :type "Array of /Game/BluePrint/VR_Inven/SlotInfo Structure") (AfterInfo :type "Array of /Game/BluePrint/VR_Inven/SlotInfo Structure") (CompareID :type Integer :default -1) (Index :type Integer) (Find :type "/Game/BluePrint/VR_Inven/SlotInfo Structure") (CompareInfo :type "/Game/BluePrint/VR_Inven/SlotInfo Structure"))
  (bind _find_item (break `/Game/BluePrint/VR_Inven/SlotInfo` (`local.Find`)))
  (bind _find_item_2 (break `/Game/BluePrint/VR_Inven/SlotInfo` (`local.Find`)))
  (bind _compareinfo_item (break `/Game/BluePrint/VR_Inven/SlotInfo` (`local.CompareInfo`)))
  (bind (_find_item_3 _find_amount) (break `/Game/BluePrint/VR_Inven/SlotInfo` (`local.Find`)))
  (bind (_compareinfo_item_2 _compareinfo_amount) (break `/Game/BluePrint/VR_Inven/SlotInfo` (`local.CompareInfo`)))
  (bind _compareinfo_item_3 (break `/Game/BluePrint/VR_Inven/SlotInfo` (`local.CompareInfo`)))
  (bind _afterinfo (`local.AfterInfo`))
  (bind (_basicinfo_type _basicinfo_id) (break `/Game/BluePrint/VR_Inven/Items/Item_BasicInfo` (`/Game/BluePrint/VR_Inven/Items/ItemBase.BasicInfo` _compareinfo_item)))
  (bind (_basicinfo_type_2 _basicinfo_id_2) (break `/Game/BluePrint/VR_Inven/Items/Item_BasicInfo` (`/Game/BluePrint/VR_Inven/Items/ItemBase.BasicInfo` _find_item_2)))
  (bind (_basicinfo_type_3 _basicinfo_id_3) (break `/Game/BluePrint/VR_Inven/Items/Item_BasicInfo` (`/Game/BluePrint/VR_Inven/Items/ItemBase.BasicInfo` _compareinfo_item_3)))
  ;[1 1 1] 빈슬롯이 아닌 슬롯의 Info를 저장
  (for _array_element (`self.Slots`)
    (if (not (`/Game/BluePrint/VR_Inven/VR_InvenSlot.IsEmpty` _array_element))
      (`KismetArrayLibrary.Array_Add` (`local.BeforeInfo`) (`/Game/BluePrint/VR_Inven/VR_InvenSlot.SlotInfo` _array_element))))
  ;[1 1 1] 소팅 전 배열과, 소팅 후 배열의 크기가 같을 때까지 반복
  (while (!= (`KismetArrayLibrary.Array_Length` (`local.BeforeInfo`)) (`KismetArrayLibrary.Array_Length` (`local.AfterInfo`)))
    (for (_array_element_2 _array_index) (`local.BeforeInfo`)
      (`/Engine/EditorBlueprintResources/StandardMacros.IsValid` (`.Item_3_7DCF77FE4EC0FE901CF57A9A3899E4A2` (break `/Game/BluePrint/VR_Inven/SlotInfo` _array_element_2))
        (:`Is Valid`
          (set `local.CompareInfo` _array_element_2)
          (`/Engine/EditorBlueprintResources/StandardMacros.IsValid` _find_item
            (:`Is Valid`
              ;;[1 1 1] 현재 Item과 이전에 찾은Item이 같은지 확인
              (if (== _basicinfo_id_2 _basicinfo_id)
                ;;[1 1 1] 같을 경우 갯수가 많은것으로 설정한다
                (if (>= _find_amount _compareinfo_amount)
                  (set `local.Index` _array_index)
                  (set `local.Find` (`local.CompareInfo`)))
                (else
                  ;;[1 1 1] 찾은 Item 설정
                  (if (>= _basicinfo_id_3 (`local.CompareID`)) :!label _label
                    (set `local.CompareID` _basicinfo_id_3)
                    (set `local.Index` _array_index)
                    (set `local.Find` (`local.CompareInfo`))))))
            (:`Is Not Valid`
              (goto _label))))))
    ;[1 0 0.4829] 위에서 찾은 Info를 소팅할 배열에 추가해주고 소팅 전 배열에서 지워준다
    (`KismetArrayLibrary.Array_Add` (`local.AfterInfo`) (`local.Find`))
    (`KismetArrayLibrary.Array_Set` (`local.BeforeInfo`) (`local.Index`) (make `/Game/BluePrint/VR_Inven/SlotInfo` null))
    ;;[1 1 1] 비교변수들 초기화
    (set `local.CompareID` 0)
    (set `local.Index` 0)
    (set `local.Find` (struct)))
  ;[1 1 1] 소팅된 배열을 인벤토리에 적용
  ;;[1 1 1] 먼저 슬롯을 모두 비움
  (for _array_element_3 (`self.Slots`)
    (`/Game/BluePrint/VR_Inven/VR_InvenSlot.MakeEmpty` _array_element_3))
  ;;[1 1 1] 소팅된 배열의 순서대로 슬롯에 아이템 및 갯수 설정
  (for (_array_element_4 _array_index_2) _afterinfo
    (bind (_item _amount) (break `/Game/BluePrint/VR_Inven/SlotInfo` _array_element_4))
    (`/Game/BluePrint/VR_Inven/VR_InvenSlot.SetItemAndAmount` (`KismetArrayLibrary.Array_Get` (`self.Slots`) (- (- (`KismetArrayLibrary.Array_Length` _afterinfo) 1) _array_index_2)) _item _amount)))

(fn `SortAll`
  (locals (AfterSortArray :type "Array of /Game/BluePrint/VR_Inven/SlotInfo Structure") (BeforeSortArray :type "Array of /Game/BluePrint/VR_Inven/SlotInfo Structure") (CompareInfo :type "/Game/BluePrint/VR_Inven/SlotInfo Structure") (FindInfo :type "/Game/BluePrint/VR_Inven/SlotInfo Structure") (CompareID :type Integer) (Index :type Integer))
  (bind _compareinfo_item (break `/Game/BluePrint/VR_Inven/SlotInfo` (`local.CompareInfo`)))
  (bind (_compareinfo_item_2 _compareinfo_amount) (break `/Game/BluePrint/VR_Inven/SlotInfo` (`local.CompareInfo`)))
  (bind _compareinfo_item_3 (break `/Game/BluePrint/VR_Inven/SlotInfo` (`local.CompareInfo`)))
  (bind _findinfo_item (break `/Game/BluePrint/VR_Inven/SlotInfo` (`local.FindInfo`)))
  (bind _findinfo_item_2 (break `/Game/BluePrint/VR_Inven/SlotInfo` (`local.FindInfo`)))
  (bind (_findinfo_item_3 _findinfo_amount) (break `/Game/BluePrint/VR_Inven/SlotInfo` (`local.FindInfo`)))
  (bind _aftersortarray (`local.AfterSortArray`))
  (bind _allslots (`self.AllSlots`))
  (bind (_basicinfo_type _basicinfo_id) (break `/Game/BluePrint/VR_Inven/Items/Item_BasicInfo` (`/Game/BluePrint/VR_Inven/Items/ItemBase.BasicInfo` _compareinfo_item)))
  (bind (_basicinfo_type_2 _basicinfo_id_2) (break `/Game/BluePrint/VR_Inven/Items/Item_BasicInfo` (`/Game/BluePrint/VR_Inven/Items/ItemBase.BasicInfo` _findinfo_item_2)))
  (bind (_basicinfo_type_3 _basicinfo_id_3) (break `/Game/BluePrint/VR_Inven/Items/Item_BasicInfo` (`/Game/BluePrint/VR_Inven/Items/ItemBase.BasicInfo` _compareinfo_item_3)))
  ;[1 1 1] 비어있지 않은 슬롯을 BeforeArray에 Add
  (for _array_element (`self.AllSlots`)
    (if (not (`/Game/BluePrint/VR_Inven/Items/CommonItemFunction.IsEmpty` _array_element))
      (`KismetArrayLibrary.Array_Add` (`local.BeforeSortArray`) _array_element)))
  ;[1 1 1] AfterArray에 순서대로 Add
  (while (!= (`KismetArrayLibrary.Array_Length` (`local.BeforeSortArray`)) (`KismetArrayLibrary.Array_Length` (`local.AfterSortArray`)))
    (for (_array_element_2 _array_index) (`local.BeforeSortArray`)
      (`/Engine/EditorBlueprintResources/StandardMacros.IsValid` (`.Item_3_7DCF77FE4EC0FE901CF57A9A3899E4A2` (break `/Game/BluePrint/VR_Inven/SlotInfo` _array_element_2))
        (:`Is Valid`
          (set `local.CompareInfo` _array_element_2)
          (`/Engine/EditorBlueprintResources/StandardMacros.IsValid` _findinfo_item
            (:`Is Valid`
              (if (== _basicinfo_id_2 _basicinfo_id)
                (if (>= _findinfo_amount _compareinfo_amount)
                  (set `local.Index` _array_index)
                  (set `local.FindInfo` (`local.CompareInfo`)))
                (else
                  (if (>= _basicinfo_id_3 (`local.CompareID`)) :!label _label
                    (set `local.CompareID` _basicinfo_id_3)
                    (set `local.Index` _array_index)
                    (set `local.FindInfo` (`local.CompareInfo`))))))
            (:`Is Not Valid`
              (goto _label))))))
    (`KismetArrayLibrary.Array_Add` (`local.AfterSortArray`) (`local.FindInfo`))
    (`KismetArrayLibrary.Array_Set` (`local.BeforeSortArray`) (`local.Index`) (make `/Game/BluePrint/VR_Inven/SlotInfo` null))
    (set `local.CompareID` 0)
    (set `local.Index` 0)
    (set `local.FindInfo` (make `/Game/BluePrint/VR_Inven/SlotInfo` null)))
  ;[1 1 1] 기존Array 클리어후 리사이즈
  (`KismetArrayLibrary.Array_Clear` _allslots)
  (`KismetArrayLibrary.Array_Resize` _allslots (* (`self.SlotNumPerPage`) (`self.MaxPage`)))
  ;[1 1 1] AfterSortArray에 있는 것을 기존 Array에 설정
  (for (_array_element_3 _array_index_2) _aftersortarray
    (`KismetArrayLibrary.Array_Set` (`self.AllSlots`) (- (- (`KismetArrayLibrary.Array_Length` _aftersortarray) 1) _array_index_2) _array_element_3))
  ;[1 1 1] 마무리
  (`self.UpdatePage`))

(fn `UpdatePage`
  (for (_array_element _array_index) (`self.Slots`)
    (bind (_item _amount) (break `/Game/BluePrint/VR_Inven/SlotInfo` (`KismetArrayLibrary.Array_Get` (`self.AllSlots`) (+ _array_index (* (`self.SlotNumPerPage`) (`self.CurrentPage`))))))
    (`/Game/BluePrint/VR_Inven/VR_InvenSlot.SetItemAndAmount` _array_element _item _amount)))

(fn `UserConstructionScript`)