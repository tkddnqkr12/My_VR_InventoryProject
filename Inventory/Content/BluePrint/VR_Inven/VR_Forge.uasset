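; VR forge inventory that crafts items from the materials placed in its slots and sets up left and right button bindings at start.
; Combine requires an empty player inventory slot, then takes the first CombinationList data table recipe whose every resource is met by a single slot holding enough of that item.
; It then removes the resources from matching forge slots and adds the ItemDBManager-resolved result to the player's inventory.
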(event `self.ReceiveBeginPlay`
  (`self.ConstructInven`)
  (add `self.LeftButton` (`|CreateDelegate` :!event `Combine`))
  (add `self.RightButton` (`|CreateDelegate` :!event `SortAll`)))

(fn `CheckAllTrue`
  (params (CheckList :type "Array of Boolean"))
  (returns (Result :type Boolean))
  ;[1 1 1] BoolArray가 모두 True인지 확인한다
  (for _array_element CheckList
    (if (not _array_element)
      (return false)))
  (return true))

(fn `CheckContatinResource`
  (params (Elenment :type "/Game/BluePrint/VR_Inven/Items/CombinationElement Structure"))
  (returns (Success :type Boolean))
  (bind (_itemid _amount) (break `/Game/BluePrint/VR_Inven/Items/CombinationElement` Elenment))
  ;[1 1 1] 해당 재료가 있는지, 있다면 갯수가 충분한지 확인
  (for _array_element (`self.AllSlots`)
    (if (not (`/Game/BluePrint/VR_Inven/Items/CommonItemFunction.IsEmpty` _array_element))
      (bind (_item _amount_2) (break `/Game/BluePrint/VR_Inven/SlotInfo` _array_element))
      (bind (_basicinfo_type _basicinfo_id) (break `/Game/BluePrint/VR_Inven/Items/Item_BasicInfo` (`/Game/BluePrint/VR_Inven/Items/ItemBase.BasicInfo` _item)))
      (if (and (== _basicinfo_id _itemid) (>= _amount_2 _amount))
        (return true))))
  (return false))

(fn `Combine`
  ;[1 1 1] 플레이어Inventory에 빈칸이 있을 때만 진행
  (bind _success (`self.GetEmptySlot` (`self.PlayerInventory`)))
  (if _success
    ;[1 1 1] 적당한 Recipe찾음
    (bind (_success_2 _combinationrecipe) (`self.FindProperRecipe`))
    (if _success_2
      ;[1 1 1] 찾았다면 재료 소모
      (`self.ConsumeResource` _combinationrecipe)
      (bind (_resources _resultitemid _resultamount) (break `/Game/BluePrint/VR_Inven/Items/CombinationRecipe` _combinationrecipe))
      ;[1 1 1] 결과물을 플레이어 인벤토리에 추가해준다
      (`self.AddItem` (`self.PlayerInventory`) (`.Item` (`/Game/BluePrint/VR_Inven/Items/ItemDBManager.GetItemByID` (`self.ItemDBManager`) _resultitemid)) _resultamount))))

(fn `ConsumeResource`
  (params (Recipe :type "/Game/BluePrint/VR_Inven/Items/CombinationRecipe Structure"))
  ;[1 1 1] 찾은 Recipe대로 필요 아이템을 필요 갯수만큼 사용한다
  (for (_array_element _array_index) (`self.AllSlots`)
    (if (not (`/Game/BluePrint/VR_Inven/Items/CommonItemFunction.IsEmpty` _array_element))
      (for _array_element_2 (`.Resources_4_29D360E74C9048CE3C0EF89A8B2151EA` (break `/Game/BluePrint/VR_Inven/Items/CombinationRecipe` Recipe))
        (bind (_itemid _amount) (break `/Game/BluePrint/VR_Inven/Items/CombinationElement` _array_element_2))
        (bind (_basicinfo_type _basicinfo_id) (break `/Game/BluePrint/VR_Inven/Items/Item_BasicInfo` (`/Game/BluePrint/VR_Inven/Items/ItemBase.BasicInfo` (`.Item_3_7DCF77FE4EC0FE901CF57A9A3899E4A2` (break `/Game/BluePrint/VR_Inven/SlotInfo` _array_element)))))
        (if (== _itemid _basicinfo_id)
          (`self.RemoveItem` (`.Item` (`/Game/BluePrint/VR_Inven/Items/ItemDBManager.GetItemByID` (`self.ItemDBManager`) _itemid)) _array_index _amount)
          (break))))))

(fn `FindProperRecipe`
  (returns (Success :type Boolean) (CombinationRecipe :type "/Game/BluePrint/VR_Inven/Items/CombinationRecipe Structure"))
  (locals (Find :type Boolean) (FindCombination :type "/Game/BluePrint/VR_Inven/Items/CombinationRecipe Structure") (TotalList :type "Array of Boolean"))
  (bind _totallist (`local.TotalList`))
  ;[1 1 1] 데이터 테이블에서 현재 슬롯에 있는 아이템들로 만들수 있는 Recipe를 반환한다
  (bind _outrownames (`DataTableFunctionLibrary.GetDataTableRowNames` "/Game/BluePrint/VR_Inven/Items/CombinationList.CombinationList"))
  (for _array_element _outrownames
    (bind _returnvalue (`|GetDataTableRow` "/Game/BluePrint/VR_Inven/Items/CombinationList.CombinationList" _array_element)
      (:`then`
        (for _array_element_2 (`.Resources_4_29D360E74C9048CE3C0EF89A8B2151EA` (break `/Game/BluePrint/VR_Inven/Items/CombinationRecipe` _returnvalue))
          (bind _success (`self.CheckContatinResource` _array_element_2))
          (`KismetArrayLibrary.Array_Add` (`local.TotalList`) _success))
        (if (`self.CheckAllTrue` (`local.TotalList`))
          (set `local.FindCombination` _returnvalue)
          (set `local.Find` true)
          (break)
          (else
            (`KismetArrayLibrary.Array_Clear` _totallist)
            (`KismetArrayLibrary.Array_Resize` _totallist))))))
  (return (`local.Find`) (`local.FindCombination`)))

(fn `UserConstructionScript`
  (`parent.UserConstructionScript`))