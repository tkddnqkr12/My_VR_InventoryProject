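; VR inventory slot that holds an item and amount, shown through background and icon sprites plus a text render for the count.
; Controller hover registers the slot as HoveredSlot, swaps the background sprite and plays a timeline that scales the icon; ending hover clears both.
; Setter functions update SlotInfo and visuals together, with IsEmpty and IsFull checks against the item and its max capacity.
; OnSlotUse is an empty event.
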(event `self.ReceiveBeginPlay`
  (`PrimitiveComponent.SetCastShadow` (`self.BackGround`) false)
  (`PrimitiveComponent.SetCastShadow` (`self.Icon`) false)
  (`PrimitiveComponent.SetCastShadow` (`self.TextRender`) false))

(event `OnHover`
  (params (Controller :type "/Game/VirtualRealityBP/Blueprints/BP_MotionController Object Reference"))
  (set `/Game/VirtualRealityBP/Blueprints/BP_MotionController.HoveredSlot` self Controller)
  (`PaperSpriteComponent.SetSprite` (`self.BackGround`) "/Game/Resource/Sprites/Slot_Hovered_Sprite.Slot_Hovered_Sprite")
  (bind (_direction `_새_트랙_0`) (`Timeline|타임라인_0` :!via `PlayFromStart`)
    (:`Update`
      (`SceneComponent.SetRelativeScale3D` (`self.Icon`) (`KismetMathLibrary.MakeVector` `_새_트랙_0` 0.0 `_새_트랙_0`)))))

(event `EndHover`
  (params (Controller :type "/Game/VirtualRealityBP/Blueprints/BP_MotionController Object Reference"))
  (set `/Game/VirtualRealityBP/Blueprints/BP_MotionController.HoveredSlot` null Controller)
  (`PaperSpriteComponent.SetSprite` (`self.BackGround`) "/Game/Resource/Sprites/Slot_Sprite.Slot_Sprite"))

(event `OnSlotUse`)

(fn `AddAmount`
  (params (Add :type Integer))
  (bind _structout (setmembers `/Game/BluePrint/VR_Inven/SlotInfo` :`StructRef` (`self.SlotInfo`) :`Amount` (+ Add (`.Amount_5_09D7E4E74F30AAC3887F9490B13706AF` (break `/Game/BluePrint/VR_Inven/SlotInfo` (`self.SlotInfo`))))))
  (`TextRenderComponent.K2_SetText` (`self.TextRender`) (`KismetTextLibrary.Conv_IntToText` (`.Amount_5_09D7E4E74F30AAC3887F9490B13706AF` (break `/Game/BluePrint/VR_Inven/SlotInfo` _structout)))))

(fn `IsEmpty`
  (returns (Empty :type Boolean))
  (return (not (`KismetSystemLibrary.IsValid` (`.Item_3_7DCF77FE4EC0FE901CF57A9A3899E4A2` (break `/Game/BluePrint/VR_Inven/SlotInfo` (`self.SlotInfo`)))))))

(fn `IsFull`
  (returns (Full :type Boolean))
  (bind (_item _amount) (break `/Game/BluePrint/VR_Inven/SlotInfo` (`self.SlotInfo`)))
  (`/Engine/EditorBlueprintResources/StandardMacros.IsValid` _item
    (:`Is Valid`
      (return (== (`.MaxCapacity_12_63BD25A44B57E528AF009DB7EEAA147F` (break `/Game/BluePrint/VR_Inven/Items/Item_BasicInfo` (`/Game/BluePrint/VR_Inven/Items/ItemBase.BasicInfo` _item))) _amount)))
    (:`Is Not Valid`
      (return false))))

(fn `MakeEmpty`
  (`self.SetNewItem` null))

(fn `PrintSlotInfo`
  (params (Duration :type "Float (double-precision)"))
  (bind (_item _amount) (break `/Game/BluePrint/VR_Inven/SlotInfo` (`self.SlotInfo`)))
  (`/Engine/EditorBlueprintResources/StandardMacros.IsValid` _item
    (:`Is Valid`
      (`/Game/BluePrint/VR_Inven/Items/CommonItemFunction.PrintBasicInfo` (`/Game/BluePrint/VR_Inven/Items/ItemBase.BasicInfo` _item) Duration)
      (`KismetSystemLibrary.PrintString` (`KismetStringLibrary.Concat_StrStr` "Amount : " (`KismetStringLibrary.Conv_IntToString` _amount)) true true (struct :`G` 0.66 :`B` 1.0 :`A` 1.0) Duration))))

(fn `SetAmount`
  (params (Amount :type Integer))
  (bind _structout (setmembers `/Game/BluePrint/VR_Inven/SlotInfo` :`StructRef` (`self.SlotInfo`) :`Amount` Amount))
  (`TextRenderComponent.K2_SetText` (`self.TextRender`) (`KismetTextLibrary.Conv_IntToText` (`.Amount_5_09D7E4E74F30AAC3887F9490B13706AF` (break `/Game/BluePrint/VR_Inven/SlotInfo` _structout)))))

(fn `SetItemAndAmount`
  (params (Item :type "/Game/BluePrint/VR_Inven/Items/ItemBase Object Reference") (Amount :type Integer))
  (bind _icon (`self.Icon`))
  (bind _icon_2 (`self.Icon`))
  (`/Engine/EditorBlueprintResources/StandardMacros.IsValid` Item
    (:`Is Valid`
      (bind _structout (setmembers `/Game/BluePrint/VR_Inven/SlotInfo` :`StructRef` (`self.SlotInfo`) :`Item` Item :`Amount` Amount))
      (bind (_item _amount) (break `/Game/BluePrint/VR_Inven/SlotInfo` _structout))
      (bind (_type _id _name _description _category _rarity _maxcapacity _icon_3 _iconcolor) (break `/Game/BluePrint/VR_Inven/Items/Item_BasicInfo` (`/Game/BluePrint/VR_Inven/Items/ItemBase.BasicInfo` _item)))
      (`PaperSpriteComponent.SetSprite` _icon_2 _icon_3)
      (`PaperSpriteComponent.SetSpriteColor` _icon_2 _iconcolor)
      (`TextRenderComponent.K2_SetText` (`self.TextRender`) (`KismetTextLibrary.Conv_IntToText` _amount)))
    (:`Is Not Valid`
      (`PaperSpriteComponent.SetSprite` _icon null)
      (`PaperSpriteComponent.SetSpriteColor` :`self` _icon)
      (`TextRenderComponent.K2_SetText` (`self.TextRender`) ""))))

(fn `SetNewItem`
  (params (NewItem :type "/Game/BluePrint/VR_Inven/Items/ItemBase Object Reference"))
  (bind _icon (`self.Icon`))
  (bind _slotinfo (`self.SlotInfo`))
  (`/Engine/EditorBlueprintResources/StandardMacros.IsValid` NewItem
    (:`Is Valid`
      (bind _structout (setmembers `/Game/BluePrint/VR_Inven/SlotInfo` :`StructRef` _slotinfo :`Item` NewItem :`Amount` 0))
      (bind (_type _id _name _description _category _rarity _maxcapacity _icon_2 _iconcolor) (break `/Game/BluePrint/VR_Inven/Items/Item_BasicInfo` (`/Game/BluePrint/VR_Inven/Items/ItemBase.BasicInfo` (`.Item_3_7DCF77FE4EC0FE901CF57A9A3899E4A2` (break `/Game/BluePrint/VR_Inven/SlotInfo` _structout)))))
      (`PaperSpriteComponent.SetSprite` _icon _icon_2)
      (`PaperSpriteComponent.SetSpriteColor` _icon _iconcolor)
      (`TextRenderComponent.K2_SetText` (`self.TextRender`) (`KismetTextLibrary.Conv_IntToText` 0)))
    (:`Is Not Valid`
      (setmembers `/Game/BluePrint/VR_Inven/SlotInfo` :`StructRef` _slotinfo :`Item` null :`Amount` 0)
      (`PaperSpriteComponent.SetSprite` (`self.Icon`) null)
      (`TextRenderComponent.K2_SetText` (`self.TextRender`) ""))))

(fn `UserConstructionScript`)