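; ItemSearch provides lookup helpers for inventory items stored in ItemDataTable.
; GetItemByID and GetItemByName linearly scan every row and return the first match on the ID or Name field, rather than keying on row name.
; When nothing matches, both return without setting an item.
; PrintItem is a debug helper that prints an item's category, type, description, name and ID.
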(fn `GetItemByID`
  (params (ID :type Integer))
  (returns (ItemInfo :type "/Game/BluePrint/NormalInven/ItemStruct Structure"))
  (bind _outrownames (`DataTableFunctionLibrary.GetDataTableRowNames` "/Game/BluePrint/NormalInven/ItemDataTable.ItemDataTable"))
  (for _array_element _outrownames
    (bind _returnvalue (`|GetDataTableRow` "/Game/BluePrint/NormalInven/ItemDataTable.ItemDataTable" _array_element)
      (:`then`
        (if (== (`.ID_2_C0344EE94A6EEC65B57F0CB0DC50418A` (break `/Game/BluePrint/NormalInven/ItemStruct` _returnvalue)) ID)
          (return _returnvalue)))))
  (return))

(fn `GetItemByName`
  (params (Name :type Name))
  (returns (ItemInfo :type "/Game/BluePrint/NormalInven/ItemStruct Structure"))
  (bind _outrownames (`DataTableFunctionLibrary.GetDataTableRowNames` "/Game/BluePrint/NormalInven/ItemDataTable.ItemDataTable"))
  (for _array_element _outrownames
    (bind _returnvalue (`|GetDataTableRow` "/Game/BluePrint/NormalInven/ItemDataTable.ItemDataTable" _array_element)
      (:`then`
        (if (== (`.Name_26_62EEA5754AA78C7B7FEE4E8092E427EB` (break `/Game/BluePrint/NormalInven/ItemStruct` _returnvalue)) Name)
          (return _returnvalue)))))
  (return))

(fn `PrintItem`
  (params (Item :type "/Game/BluePrint/NormalInven/ItemStruct Structure"))
  (bind (_id _name _description _type _category) (break `/Game/BluePrint/NormalInven/ItemStruct` Item))
  (`KismetSystemLibrary.PrintString` null (`|GetEnumeratorNameAsString` _category) true true (struct :`R` 1.0 :`B` 0.141263 :`A` 1.0) 10.0)
  (`KismetSystemLibrary.PrintString` null (`|GetEnumeratorNameAsString` _type) true true (struct :`R` 1.0 :`B` 0.141263 :`A` 1.0) 10.0)
  (`KismetSystemLibrary.PrintString` null _description true true (struct :`R` 1.0 :`B` 0.141263 :`A` 1.0) 10.0)
  (`KismetSystemLibrary.PrintString` null (`KismetStringLibrary.Conv_NameToString` _name) true true (struct :`R` 1.0 :`B` 0.141263 :`A` 1.0) 10.0)
  (`KismetSystemLibrary.PrintString` null (`KismetStringLibrary.Conv_IntToString` _id) true true (struct :`R` 1.0 :`B` 0.141263 :`A` 1.0) 10.0))